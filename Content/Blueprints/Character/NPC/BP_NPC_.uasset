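; NPC Blueprint that takes point damage and dies when its Health runs out.
; Death passes from a request event to a multicast-named event that ragdolls the mesh, disables capsule collision and changes NPC state.
; That event also reports the hit bone to a player damage causer for kill feedback.
; A death montage branch is left disconnected, and an uncalled helper macro separates server, local client and other clients.
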(event Custom|Dead_Req
  (params (DamageCauser :type Actor%20Object%20Reference) (BoneName :type Name))
  (CallFunction|DeadMultacast DamageCauser BoneName))

(event Custom|Dead_Multacast
  (params (DamageCauser :type Actor%20Object%20Reference) (BoneName :type Name))
  (Physics|SetSimulatePhysics (Variables|Character|GetMesh) true)
  (Collision|SetCollisionEnabled (Variables|Collision|GetCapsuleComponent) "NoCollision")
  (Variables|Default|SetNPCState "NewEnumerator1")
  (bind _asbp_player_character (Utilities|Casting|CastToBP_PlayerCharacter DamageCauser))
  (Development|PrintString "kill")
  (Default|KillFeedBackReq _asbp_player_character BoneName))

(event EventBeginPlay)

(event Collision|EventActorBeginOverlap
  (params (OtherActor :type Actor%20Object%20Reference)))

(event EventTick
  (params (DeltaSeconds :type Float%20%28single-precision%29)))

(event Game|Damage|EventAnyDamage
  (params (Damage :type Float%20%28single-precision%29) (DamageType :type Damage%20Type%20Object%20Reference) (InstigatedBy :type Controller%20Object%20Reference) (DamageCauser :type Actor%20Object%20Reference)))

(event Game|Damage|EventPointDamage
  (params (Damage :type Float%20%28single-precision%29) (DamageType :type Damage%20Type%20Object%20Reference) (HitLocation :type Vector :default "0, 0, 0") (HitNormal :type Vector :default "0, 0, 0") (HitComponent :type Primitive%20Component%20Object%20Reference) (BoneName :type Name :default "None") (ShotFromDirection :type Vector :default "0, 0, 0") (InstigatedBy :type Controller%20Object%20Reference) (DamageCauser :type Actor%20Object%20Reference) (HitInfo :type Hit%20Result%20Structure%20%28by%20ref%29))
  (Variables|Default|SetHealth (- (Variables|Default|GetHealth) Damage))
  (if (<= (Variables|Default|GetHealth) 0.0)
    (CallFunction|DeadReq DamageCauser BoneName)))

(fn ConstructionScript)