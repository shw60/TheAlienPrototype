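; BP_Frag is a thrown frag grenade that explodes on a timed fuse.
; Throw sets the projectile movement velocity and activates it, then after a short delay spawns BP_Explosion at the grenade's transform and hides the mesh.
; A lifespan set slightly longer than the fuse destroys the actor just after detonation.
; Inline explosion sound, particle and smoke chains remain in the graph but are disconnected.
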(event Custom|Throw
  (params (Velocity :type Vector))
  (bind _projectilemovement (Variables|Default|GetProjectileMovement))
  (Variables|/Script/Engine.MovementComponent|SetVelocity _projectilemovement Velocity)
  (Components|Activation|Activate _projectilemovement false)
  (Actor|SetLifeSpan 2.1)
  (Utilities|FlowControl|Delay 2.0)
  (Game|SpawnActorfromClass "/Game/Blueprints/Item/Weapon/BP_Explosion.BP_Explosion_C" (Transformation|GetActorTransform) "Undefined" 0 0)
  (Development|SetHiddeninGame (Variables|Default|GetGrenadeMesh) true false))

(event EventBeginPlay)

(event Collision|EventActorBeginOverlap
  (params (OtherActor :type Actor%20Object%20Reference)))

(event EventTick
  (params (DeltaSeconds :type Float%20%28single-precision%29)))

(fn ConstructionScript)