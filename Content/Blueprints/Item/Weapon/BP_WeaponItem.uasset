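; BP_WeaponItem is a weapon item actor that sets up its mesh from data.
; On BeginPlay, a nonzero ItemID is converted to a row name and looked up in the weapon data table.
; The found row's static mesh is async loaded and assigned to the StaticMesh component once loading completes.
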(event EventBeginPlay
  (if (!= (Variables|Default|GetItemID) 0)
    (bind _returnvalue (Utilities|GetDataTableRow "/Game/GameData/WeaponDAtaTable.WeaponDataTable" (Utilities|String|StringToName (Utilities|String|ToString(Integer) (Variables|Default|GetItemID))))
      (:then
        (bind _object (Utilities|AsyncLoadAsset (.StaticMesh (Utilities|Struct|BreakWeaponClass _returnvalue)))
          (:Completed
            (bind _asstatic_mesh (Utilities|Casting|CastToStaticMesh _object))
            (Components|StaticMesh|SetStaticMesh (Variables|Default|GetStaticMesh) _asstatic_mesh)))))))

(fn ConstructionScript)